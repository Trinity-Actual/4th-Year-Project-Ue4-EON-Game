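; Main controller for a network spectrum-assignment game, driving the BP_UI_HUD connection request list and three-panel navigation.
; BeginPlay creates the HUD, caches its widgets in arrays and hides all nine request slots.
; Test keys F and G add randomised source/destination/slot-count requests and remove them (removal is flagged buggy).
; Tick moves panel highlight via Enter/Backspace and ends play when GameModeTimers hits zero, enabling gated R-key level restart.
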(event Custom|Display%20Connection%20Slot
  (params (Slot_REF_Index :type Integer))
  ;[1 1 1] Function To Display New Connection Request
  (Widget|SetVisibility (Utilities|Array|Get(acopy) (Variables|Default|GetSlot_REF_Array) Slot_REF_Index) "Visible")
  (Default|SetConnectionInfo (Variables|Default|GetHUD_REF) (Utilities|Array|Get(acopy) (Variables|Default|GetSrc_Node_REF) Slot_REF_Index) (Utilities|Array|Get(acopy) (Variables|Default|GetDest_Node_REF) Slot_REF_Index) (Utilities|Array|Get(acopy) (Variables|Default|GetSpectrumSlot_Num) Slot_REF_Index) (Variables|Default|GetSrc_Node) (Variables|Default|GetDest_Node) (Variables|Default|GetSlots)))

(event Custom|UI%20Switch
  ;[1 1 1] Function to Switch UI Selected Based on User Input
  (bind _output_get (Variables|Default|SetUI_Switch_REF_Array (Variables|Default|GetUI_Switch_REF_Array)))
  (Class|Border|SetBrushColor _output_get "(R=0.300000,G=0.300000,B=0.300000,A=1.000000)")
  (Class|Border|SetBrushColor (Utilities|Array|Get(acopy) (Variables|Default|GetUI_Switch_REF_Array) (Math|Conversions|ToInteger(Byte) (Variables|Default|GetUI_Status_Enum))) "(R=1.000000,G=0.000000,B=0.000000,A=1.000000)"))

(event Custom|Hide%20Connection%20Slot
  (params (Slot%20REF%20Index :type Integer))
  ;[1 1 1] Function to Hide Connection Slot
  (Widget|SetVisibility (Utilities|Array|Get(acopy) (Variables|Default|GetSlot_REF_Array) Slot%20REF%20Index) "Hidden"))

(event Custom|New%20Connection%20Request
  (bind _is_slot_visible (Variables|Default|GetIs_Slot_Visible))
  ;[1 1 1] Creating New Connection Request with random source and destination nodes and number of spectrum slots required.
  ; TO DO: Add condition that if source and destination node are == then do not pass the function
  (Variables|Default|SetSrc_Node (Math|Random|RandomIntegerinRange 1 5))
  (Variables|Default|SetDest_Node (Math|Random|RandomIntegerinRange 1 5))
  (Variables|Default|SetSlots (Math|Random|RandomIntegerinRange 1 6))
  (bind (_array_element _array_index) (Utilities|Array|ForEachLoopwithBreak _is_slot_visible)
    (:LoopBody
      (if (not _array_element)
        (Utilities|Array|SetArrayElem _is_slot_visible _array_index true true)
        (CallFunction|DisplayConnectionSlot _array_index)
        (CallFunction|BreakConnReqLoop)))))

(event Custom|Break%20Conn_Req%20Loop
  (bind _is_slot_visible (Variables|Default|GetIs_Slot_Visible))
  ;[1 1 1] Creating New Connection Request with random source and destination nodes and number of spectrum slots required.
  ; TO DO: Add condition that if source and destination node are == then do not pass the function
  (Utilities|Array|ForEachLoopwithBreak _is_slot_visible) ; enters at Break
)

(event Custom|Break%20hide%20Conn%20Loop
  (bind _is_slot_visible (Variables|Default|GetIs_Slot_Visible))
  (bind _is_slot_visible_2 (Variables|Default|GetIs_Slot_Visible))
  ;[1 1 1] TO DEBUG: When it hits the 9th Slot it cannot remove anymore
  (Utilities|Array|ForEachLoopwithBreak _is_slot_visible_2) ; enters at Break
)

(event EventBeginPlay
  ;[1 1 1] Game Setup Code
  (|CreateHUDWidget
    (:Next
      (|CreatingSlotAddressArray) ; Creating Slot Array Addressing for Game Mechanics
      (|HidingSlotsviacreatedArray ; Connection slots will be hidden at game initialisation
        (:Completed
          (|CreatingUIAddressArray) ; Create LCR UI Array Addressing for navigation
          (|SetLEFT_UIAsSelected) ; Puts Red Border For Left UI on Game Start
          ;[1 1 1] Additional Initialisation Arrays for Connection Slots Generation
          (|SetSpectrumSlotReferences)
          (|SetSourceNodeReferences)
          (|SetDestinationNodeReferences))))))

(event EventTick
  (params (DeltaSeconds :type Float%20%28single-precision%29))
  ;[1 1 1] Main Game Loop
  (|CheckGameOver
    (:true
      (|RestartSequence) ; Game Restart Function, executes when 'R' is pressed
    )
    (:false
      (|GetGameTime_2 ; Debug Print string for game time disconnected
        (:Game%20Time%20NOT%200
          (|GetUserUISwitchInput) ; Navigates UI USING ENUM
        )))))

(event Input|KeyboardEvents|R
  (params (Key :type Key%20Structure :default "None"))
  ;[1 1 1] Main Game Loop
  (:Pressed
    (|RestartSequence) ; enters at Open
  )
  (:Released
    (|RestartSequence) ; enters at Close
  ))

(event Input|KeyboardEvents|G
  (params (Key :type Key%20Structure :default "None"))
  (bind _is_slot_visible (Variables|Default|GetIs_Slot_Visible))
  (bind _is_slot_visible_2 (Variables|Default|GetIs_Slot_Visible))
  ;[1 1 1] TO DEBUG: When it hits the 9th Slot it cannot remove anymore
  (:Pressed
    (bind (_array_element _array_index) (Utilities|Array|ForEachLoopwithBreak _is_slot_visible_2)
      (:LoopBody
        (if _array_element
          (if (== (Class|KismetMathLibrary|ToInt64(Integer) (Utilities|Array|Length _is_slot_visible)) (Class|KismetMathLibrary|ToInt64(Integer) _array_index))
            (Utilities|Array|SetArrayElem _is_slot_visible _array_index false)
            (CallFunction|HideConnectionSlot (- _array_index 1) :!label _label)
            (CallFunction|BreakHideConnLoop))
          (else
            (Utilities|Array|SetArrayElem _is_slot_visible_2 (- _array_index 1) false true)
            (goto _label)))))))

(event Input|KeyboardEvents|F
  (params (Key :type Key%20Structure :default "None"))
  ;[1 1 1] For Testing Connection Requests
  (:Pressed
    (CallFunction|NewConnectionRequest)))

(fn ConstructionScript)

(event Input|KeyboardEvents|Escape
  (params (Key :type Key%20Structure :default "None"))
  ;[1 1 1] Moving Back through UI (Right to Left)
  (:Pressed
    (Utilities|FlowControl|Gate true) ; enters at Open
  ))

(event Input|KeyboardEvents|Enter
  (params (Key :type Key%20Structure :default "None"))
  ;[1 1 1] Moving Forward through UI (Left to Right)
  (:Pressed
    (Utilities|FlowControl|Gate true) ; enters at Open
  ))